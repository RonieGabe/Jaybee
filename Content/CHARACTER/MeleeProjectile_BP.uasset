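; Melee area-of-effect actor that damages and knocks back what its expanding cylinder overlaps.
; SetMeleeParameters stores damage, knockback and causer, assigns the effect asset, and matches effect lifetime and CylinderResize timeline rate to FXTime.
; ActivateAOE plays the timeline to scale the cylinder horizontally, then destroys it and, after a short delay, the actor.
; Overlaps send DamageEnemyMessage with the actor's root location as damage origin.
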(event `Set Melee Parameters`
  (params (DamageCauser :type "Actor Object Reference") (`(-)DamageAmount` :type "Float (double-precision)") (`FX Time` :type "Float (double-precision)") (`knockback amount` :type "Float (double-precision)") (`AoE Effect Type` :type "NiagaraSystem Object Reference"))
  (set `self.Damage Causer` DamageCauser)
  (set `self.Damage Amount` `(-)DamageAmount`)
  (set `self.Knockback Amount` `knockback amount`)
  (`FXSystemComponent.SetFloatParameter` (`self.AoE Effect`) "EffectLifeline" `FX Time`)
  (`TimelineComponent.SetPlayRate` (`self.CylinderResize`) (/ 1.0 `FX Time`))
  (`NiagaraComponent.SetAsset` (`self.AoE Effect`) `AoE Effect Type`))

(event `self.ReceiveBeginPlay`)

(event `ActivateAOE`
  (bind (_direction _cylindersize) (`Timeline|CylinderResize` :!via `PlayFromStart`)
    (:`Update`
      (`SceneComponent.SetWorldScale3D` (`self.Cylinder`) (`KismetMathLibrary.MakeVector` _cylindersize _cylindersize 1.0)))
    (:`Finished`
      (`ActorComponent.K2_DestroyComponent` (`self.Cylinder`))
      (`KismetSystemLibrary.Delay` 1.0)
      (`self.K2_DestroyActor`))))

(event `self.Cylinder.OnComponentBeginOverlap`
  (params (OverlappedComponent :type "PrimitiveComponent Object Reference") (OtherActor :type "Actor Object Reference") (OtherComp :type "PrimitiveComponent Object Reference") (OtherBodyIndex :type Integer) (bFromSweep :type Boolean) (SweepResult :type "HitResult Structure (by ref)"))
  (message `/Game/CHARACTER/CharacterInterface.Damage Enemy` OtherActor (`self.Damage Amount`) (`self.Knockback Amount`) (`SceneComponent.K2_GetComponentLocation` (`self.DefaultSceneRoot`)) (`self.Damage Causer`)))

(fn `UserConstructionScript`)