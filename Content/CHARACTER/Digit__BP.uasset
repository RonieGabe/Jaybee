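; Character Blueprint for Digit, a child fighter class with its own stamina costs, data-table skins, air special and melee hitboxes.
; The air special plays a montage, then launches Digit forward and down with locked rotation and pawn collision set to overlap.
; Right-hand and Fann overlaps, gated by can-damage flags, damage and knock back targets.
; The same hits ricochet an ungrabbed Jaybee ball away through a debounced macro.
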(event `self.ReceiveBeginPlay`
  (bind _mesh (`self.Mesh`))
  (bind _mesh_2 (`self.Mesh`))
  ;[1 1 1] set stamina stats
  (`parent.ReceiveBeginPlay`)
  (`self.Set Stats` (`self.DigitName`))
  (set `self.Dash Stamina Req` 2.0)
  (set `self.Special Stamina req` 3.0)
  ;[1 1 1] set skin
  (bind _returnvalue (`|GetDataTableRow` "/Game/CHARACTER/DataTables/SkinsDataTable.SkinsDataTable" "Digit")
    (:`then`
      (switch `int` (`self.SKIN NUMBER`)
        (:`0`
          (bind (_skin1 _skin2 _skin3 _skin4) (break `/Game/CHARACTER/DataTables/SkinStruct` _returnvalue))
          (for (_array_element _array_index) _skin1
            (`PrimitiveComponent.SetMaterial` _mesh_2 _array_index _array_element)))
        (:`1`
          (for (_array_element_2 _array_index_2) _skin2
            (`PrimitiveComponent.SetMaterial` _mesh_2 _array_index_2 _array_element_2)))
        (:`2`
          (for (_array_element_3 _array_index_3) _skin3
            (`PrimitiveComponent.SetMaterial` _mesh _array_index_3 _array_element_3)))
        (:`3`
          (for (_array_element_4 _array_index_4) _skin4
            (`PrimitiveComponent.SetMaterial` _mesh _array_index_4 _array_element_4)))))))

(event `self.Begin Air Special`
  (bind (_returnvalue_x _returnvalue_y) (`KismetMathLibrary.BreakVector` (* (`SceneComponent.GetForwardVector` (`self.CapsuleComponent`)) 3000.0)))
  (`|PlayMontage` (`self.Mesh`) (`.AirPreSpecial_11_A5B128244D932CB362577BB76BBB5B9D` (break `/Game/CHARACTER/DataTables/Montage_Struct` (`self.Montages`)))
    (:`then`
      (set `self.IsAttacking` true))
    (:`OnCompleted`
      (set `self.SpecialActive` true)
      (`self.LaunchCharacter` (`KismetMathLibrary.MakeVector` _returnvalue_x _returnvalue_y -2000.0))
      (set `CharacterMovementComponent.RotationRate` (struct) (`self.CharacterMovement`))
      (`|PlayMontage` (`self.Mesh`) "/Game/CHARACTER/DigitNEW/Digit_V2_Animations/specials/DM_SpecialAir_Start.DM_SpecialAir_Start"
        (:`then`
          (set `self.(R)Hand_CanDamage` true)
          (`PrimitiveComponent.SetCollisionResponseToChannel` (`self.CapsuleComponent`) "ECC_Pawn" "ECR_Overlap")
          (`PrimitiveComponent.SetCollisionResponseToChannel` (`self.CapsuleComponent`) "ECC_GameTraceChannel5" "ECR_Overlap"))))
    (:`OnInterrupted`
      (set `self.IsAttacking` false))))

(event `self.Digit Special Landed`
  (set `CharacterMovementComponent.RotationRate` (struct :`Yaw` 1000.0) (`self.CharacterMovement`))
  (set `self.(R)Hand_CanDamage` false))

(event `self.RightHand(BIG).OnComponentBeginOverlap`
  (params (OverlappedComponent :type "PrimitiveComponent Object Reference") (OtherActor :type "Actor Object Reference") (OtherComp :type "PrimitiveComponent Object Reference") (OtherBodyIndex :type Integer) (bFromSweep :type Boolean) (SweepResult :type "HitResult Structure (by ref)"))
  ;[1 1 1] Light and Heavy Right Hand attack usese the same capsule
  (`|ExecutionSequence`
    (:`then_0`
      (if (`self.(R)Hand(BIG)_CanDamage`)
        (`|ExecutionSequence`
          (:`then_0`
            (bind _damaged_enemy (message `/Game/CHARACTER/CharacterInterface.Get Damaged Enemy` OtherActor))
            (`self.Damage Effect` _damaged_enemy)
            (message `/Game/CHARACTER/CharacterInterface.Damage Enemy (Function)` OtherActor -80.0 1300.0 (`SceneComponent.K2_GetComponentLocation` (`self.CapsuleComponent`)) self false 0.8 0))
          (:`then_1`
            (`self.Ricochet Macro` OtherActor 3500.0)))))
    (:`then_1`
      (if (`self.(R)Hand_CanDamage`)
        (`|ExecutionSequence`
          (:`then_0`
            (`self.Ricochet Macro` OtherActor 3500.0))
          (:`then_1`
            (bind _damaged_enemy_2 (message `/Game/CHARACTER/CharacterInterface.Get Damaged Enemy` OtherActor))
            (`self.Damage Effect` _damaged_enemy_2)
            (message `/Game/CHARACTER/CharacterInterface.Damage Enemy (Function)` OtherActor -50.0 1100.0 (`SceneComponent.K2_GetComponentLocation` (`self.CapsuleComponent`)) self false 0.8 0)))))))

(event `self.Fann.OnComponentBeginOverlap`
  (params (OverlappedComponent :type "PrimitiveComponent Object Reference") (OtherActor :type "Actor Object Reference") (OtherComp :type "PrimitiveComponent Object Reference") (OtherBodyIndex :type Integer) (bFromSweep :type Boolean) (SweepResult :type "HitResult Structure (by ref)"))
  ;[1 1 1] Fann Damage
  (if (`self.Light Attack Can Damage`)
    (`|ExecutionSequence`
      (:`then_0`
        (bind _damaged_actor (message `/Game/CHARACTER/CharacterInterface.Damage Enemy (Function)` OtherActor -40.0 1200.0 (`SceneComponent.K2_GetComponentLocation` (`self.CapsuleComponent`)) self false 0.6 0))
        (`self.Damage Effect` _damaged_actor))
      (:`then_1`
        (`self.Ricochet Macro` OtherActor 3500.0)))))

(event `Damage Effect`
  (params (NewParam :type "Actor Object Reference")))

(event `Right hand Grow`
  (`SceneComponent.SetWorldScale3D` (`self.RightHand(BIG)`) (0.0 0.0 0.0))
  (`KismetSystemLibrary.Delay` 0.1)
  (`SceneComponent.SetWorldScale3D` (`self.RightHand(BIG)`) (1.0 1.0 1.0)))

(fn `Interrupted!!`
  (`parent.Interrupted!!`)
  (set `self.(R)Hand_CanDamage` false)
  (set `self.Light Attack Can Damage` false)
  (set `self.(R)Hand(BIG)_CanDamage` false))

(fn `UserConstructionScript`
  (`parent.UserConstructionScript`)
  (set `self.Fann Scale` 0.8))