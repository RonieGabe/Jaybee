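; Melee area-of-effect actor that takes a damage causer, damage, knockback, effect asset and duration from its spawner.
; ActivateAOE scales a cylinder horizontally with a timeline paced to that duration, then destroys the cylinder and, after a short delay, the actor.
; Overlap damage and effect activation are disconnected, so the cylinder deals no damage here.
; Damage-enemy functions are empty stubs.
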(event `Set Melee Parameters`
  (params (DamageCauser :type "Actor Object Reference") (`(-)DamageAmount` :type "Float (double-precision)") (`FX Time` :type "Float (double-precision)") (`knockback amount` :type "Float (double-precision)") (`AoE Effect Type` :type "NiagaraSystem Object Reference"))
  (set `self.Damage Causer` DamageCauser)
  (set `self.Damage Amount` `(-)DamageAmount`)
  (set `self.Knockback Amount` `knockback amount`)
  (`FXSystemComponent.SetFloatParameter` (`self.AoE Effect`) "EffectLifeline" `FX Time`)
  (`TimelineComponent.SetPlayRate` (`self.CylinderResize`) (/ 1.0 `FX Time`))
  (`NiagaraComponent.SetAsset` (`self.AoE Effect`) `AoE Effect Type`))

(event `self.ReceiveBeginPlay`)

(event `ActivateAOE`
  (bind (_direction _cylindersize) (`Timeline|CylinderResize` :!via `PlayFromStart`)
    (:`Update`
      (`SceneComponent.SetWorldScale3D` (`self.Cylinder`) (`KismetMathLibrary.MakeVector` _cylindersize _cylindersize 1.0)))
    (:`Finished`
      (`ActorComponent.K2_DestroyComponent` (`self.Cylinder`))
      (`KismetSystemLibrary.Delay` 1.0)
      (`self.K2_DestroyActor`))))

(event `self.Cylinder.OnComponentBeginOverlap`
  (params (OverlappedComponent :type "PrimitiveComponent Object Reference") (OtherActor :type "Actor Object Reference") (OtherComp :type "PrimitiveComponent Object Reference") (OtherBodyIndex :type Integer) (bFromSweep :type Boolean) (SweepResult :type "HitResult Structure (by ref)")))

(fn `Damage Enemy (Function)`
  (params (`(-)Damage` :type "Float (double-precision)") (`Knockback Power` :type "Float (double-precision)") (`Damage Origin` :type "Vector Structure") (`Damage Causer` :type "/Game/CHARACTER/Avatar_Parent_BP Object Reference") (`Stun??` :type Boolean) (`immobile delay` :type "Float (double-precision)") (`Hit Effect` :type Integer))
  (returns (`Damaged Actor` :type "Actor Object Reference"))
  (return null))

(fn `Get Damaged Enemy`
  (returns (`Damaged Enemy` :type "Actor Object Reference"))
  (return null))

(fn `UserConstructionScript`)