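; Echo character Blueprint, a child class that sets Echo's stats and ability stamina costs and implements its melee pulse and air special attacks.
; The air special plays a montage, then slams Echo downward with pawn collision set to overlap.
; A timeline scales the Fann mesh, whose overlaps deal knockback damage and ricochet an ungrabbed Jaybee ball via a macro.
; Melee spawns an EchoPojectile carrying damage and knockback parameters.
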(event `self.ReceiveBeginPlay`
  (`parent.ReceiveBeginPlay`)
  (`self.Set Stats` (`self.EchoName`))
  (set `self.Dash Stamina Req` 2.0)
  (set `self.Special Stamina req` 3.0))

(event `Echo Air Projectile`
  ;[1 1 1] echo air attack spawn
  (bind (_direction _cylindersize) (`Timeline|Timeline_1` :!via `PlayFromStart`)
    (:`Update`
      (bind _returnvalue (* _cylindersize (`self.Fann Scale`)))
      (`SceneComponent.SetWorldScale3D` (`self.Fann`) (`KismetMathLibrary.MakeVector` _returnvalue _returnvalue 1.0)))))

(event `self.Begin Air Special`
  (`|PlayMontage` (`self.Mesh`) (`.AirPreSpecial_11_A5B128244D932CB362577BB76BBB5B9D` (break `/Game/CHARACTER/DataTables/Montage_Struct` (`self.Montages`)))
    (:`then`
      (set `self.IsAttacking` true))
    (:`OnCompleted`
      (set `self.SpecialActive` true)
      (`self.LaunchCharacter` (0.0 0.0 -2000.0))
      (`PrimitiveComponent.SetCollisionResponseToChannel` (`self.CapsuleComponent`) "ECC_Pawn" "ECR_Overlap")
      (`PrimitiveComponent.SetCollisionResponseToChannel` (`self.CapsuleComponent`) "ECC_GameTraceChannel5" "ECR_Overlap")
      (`PrimitiveComponent.SetCollisionResponseToChannel` (`self.Capsule(PlayerTag)`) "ECC_GameTraceChannel5" "ECR_Overlap"))
    (:`OnInterrupted`
      (set `self.IsAttacking` false))))

(event `self.Fann.OnComponentBeginOverlap`
  (params (OverlappedComponent :type "PrimitiveComponent Object Reference") (OtherActor :type "Actor Object Reference") (OtherComp :type "PrimitiveComponent Object Reference") (OtherBodyIndex :type Integer) (bFromSweep :type Boolean) (SweepResult :type "HitResult Structure (by ref)"))
  ;[1 1 1] air attack damage
  (`/Engine/EditorBlueprintResources/StandardMacros.IsValid` OtherActor
    (:`Is Valid`
      (if (`self.Echo Can Air Damage`)
        (`|ExecutionSequence`
          (:`then_0`
            (`self.Ricochet Macro` OtherActor 3500.0))
          (:`then_1`
            (message `/Game/CHARACTER/CharacterInterface.Damage Enemy (Function)` OtherActor -30.0 500.0 (`SceneComponent.K2_GetComponentLocation` (`self.CapsuleComponent`)) self false)))))))

(event `echo melee projectile`
  (bind _returnvalue (`|SpawnActorFromClass` "/Game/CHARACTER/AbiltyBP/EchoPojectile.EchoPojectile_C" (`KismetMathLibrary.MakeTransform` (`SceneComponent.K2_GetComponentLocation` (`self.EchoProjectileSphere`)) (`KismetMathLibrary.Conv_VectorToRotator` (`SceneComponent.GetForwardVector` (`self.CapsuleComponent`)))) "Undefined" "OverrideRootScale" null null))
  (`/Game/CHARACTER/AbiltyBP/EchoPojectile.Set Echo Pulse Parameters` _returnvalue self -30.0 1000.0 (`SceneComponent.K2_GetComponentLocation` (`self.CapsuleComponent`))))

(fn `Interrupted!!`
  (`parent.Interrupted!!`)
  (set `self.Echo Can Air Damage` false))

(fn `UserConstructionScript`
  (`parent.UserConstructionScript`)
  (set `self.Fann Scale` 2.5))