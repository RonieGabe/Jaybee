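; Playable character Blueprint for Ohm, a child of a shared character base, with a fan melee hit, a rolling dash and special attacks.
; Fan overlaps damage enemies and knock Jaybee balls away.
; Dashing swaps the mesh for an invulnerable ball with altered movement, draining stamina until a self-rescheduling check unrolls it on release or empty bar.
; The air special launches Ohm upward, and a separate event spawns a damaging pulse AoE.
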(event `self.ReceiveBeginPlay`
  (`parent.ReceiveBeginPlay`)
  (`self.Set Stats` (`self.OhmName`))
  (set `self.Dash Stamina Req` 2.0)
  (set `self.Special Stamina req` 3.0))

(event `self.Fann.OnComponentBeginOverlap`
  (params (OverlappedComponent :type "PrimitiveComponent Object Reference") (OtherActor :type "Actor Object Reference") (OtherComp :type "PrimitiveComponent Object Reference") (OtherBodyIndex :type Integer) (bFromSweep :type Boolean) (SweepResult :type "HitResult Structure (by ref)"))
  ;[1 1 1] damage fann
  (if (`self.swing can damage`)
    (`|ExecutionSequence`
      (:`then_0`
        (bind _damaged_actor (message `/Game/CHARACTER/CharacterInterface.Damage Enemy (Function)` OtherActor -40.0 1300.0 (`SceneComponent.K2_GetComponentLocation` (`self.CapsuleComponent`)) self false))
        (`self.hit effect` _damaged_actor))
      (:`then_1`
        (`self.Ricochet Ball` OtherActor 3500.0)))))

(event `hit effect`
  (params (InputObject :type "Actor Object Reference"))
  (`/Engine/EditorBlueprintResources/StandardMacros.IsValid` InputObject
    (:`Is Valid`
      (`NiagaraFunctionLibrary.SpawnSystemAtLocation` "/Game/PFX/NiagraSystems/ToBeMade/NS_DigitHit1.NS_DigitHit1" (`self.K2_GetActorLocation` InputObject)))))

(event `self.Character Dash`
  (params (NewParam :type Boolean))
  ;[1 1 1] roll
  (set `self.button released` false)
  (set `self.IsAttacking` true)
  (if (not (`self.IsRolling`))
    (`|ExecutionSequence`
      (:`then_0`
        (`|PlayMontage` (`self.Mesh`) "/Game/CHARACTER/Ohm/OhmAnim/OM_Rollup.OM_Rollup"
          (:`OnInterrupted`
            (`self.can dash again`))
          (:`OnNotifyBegin`
            (`/Game/UI/JB_UI/StaminaBar.Start/Stop   Fill/Drain` (`self.Stamina Bar Ref`) false true 0.01)
            (`/Game/UI/JB_UI/StaminaBar.Start/Stop   Fill/Drain` (`self.Stamina Bar Ref`) true false 0.03)
            (set `self.IsRolling` true)
            (set `self.Invulnerable` true)
            (`SceneComponent.SetHiddenInGame` (`self.Mesh`) true false)
            (`SceneComponent.SetHiddenInGame` (`self.Ohm Ball`) false false)
            (`self.Change Speed Roll` (`self.ohm roll speed`) 540.0 -8.0))))
      (:`then_1`
        (`KismetSystemLibrary.Delay` 1.0)
        (set `self.can unroll(check)` true)
        (`self.can unroll check`)))))

(event `self.Dash Released`
  ;[1 1 1] roll
  (set `self.button released` true))

(event `Ohm Stop Roll`
  ;[1 1 1] roll
  (if (`self.IsRolling`)
    (set `self.can unroll(check)` false)
    (`/Game/UI/JB_UI/StaminaBar.Start/Stop   Fill/Drain` (`self.Stamina Bar Ref`) false false 0.12)
    (`/Game/UI/JB_UI/StaminaBar.Start/Stop   Fill/Drain` (`self.Stamina Bar Ref`) true true 0.12)
    (`SceneComponent.SetHiddenInGame` (`self.Mesh`) false false)
    (`SceneComponent.SetHiddenInGame` (`self.Ohm Ball`) true false)
    (`|PlayMontage` (`self.Mesh`) "/Game/CHARACTER/Ohm/OhmAnim/OM_Unroll.OM_Unroll"
      (:`then`
        (`self.Change Speed Roll` (`.Speed_2_DD82F46641FE999FFA3091B11DE6CDE6` (break `/Game/CHARACTER/DataTables/Stats_Struct` (`self.stats`))) (`self.base character turn rate`) 8.0))
      (:`OnBlendOut`
        (`/Engine/EditorBlueprintResources/StandardMacros.DoOnce` false :!label _label
          (:`Completed`
            (set `self.Invulnerable` false)
            (set `self.IsAttacking` false)
            (set `self.IsRolling` false)
            (`KismetSystemLibrary.Delay` 0.5)
            (`self.can dash again`))))
      (:`OnInterrupted`
        (goto _label))
      (:`OnNotifyBegin`
        (goto _label :!via `Reset`)))))

(event `can unroll check`
  ;[1 1 1] roll
  (if (`self.can unroll(check)`)
    (if (<= (`/Game/UI/JB_UI/StaminaBar.Bar Current Value` (`self.Stamina Bar Ref`)) 0.0)
      (`self.Ohm Stop Roll` :!label _label_2)
      (elif (`self.button released`)
        (goto _label_2)
        (else
          (`KismetSystemLibrary.Delay` 0.1)
          (`self.can unroll check`))))))

(event `self.Begin Air Special`
  (`self.LaunchCharacter` (0.0 0.0 400.0) false true)
  ;[1 1 1] air special
  (`|PlayMontage` (`self.Mesh`) (`.AirPreSpecial_11_A5B128244D932CB362577BB76BBB5B9D` (break `/Game/CHARACTER/DataTables/Montage_Struct` (`self.Montages`)))
    (:`then`
      (set `self.IsAttacking` true))
    (:`OnCompleted`
      (set `self.IsAttacking` false :!label _label_3)
      (`KismetSystemLibrary.RetriggerableDelay` 0.03)
      (`self.can special again`))
    (:`OnInterrupted`
      (goto _label_3))))

(event `Ohm Spawn AOE`
  ;[1 1 1] spawn aoe
  (bind _returnvalue (`|SpawnActorFromClass` "/Game/CHARACTER/AbiltyBP/AoE_Sphere.AoE_Sphere_C" (`KismetMathLibrary.MakeTransform` (`SceneComponent.K2_GetComponentLocation` (`self.Mesh`))) "Undefined" "OverrideRootScale" null null))
  (`/Game/CHARACTER/AbiltyBP/AoE_Sphere.Set AoE Parameters` _returnvalue self -2.0 0.3 400.0 "/Game/PFX/NiagraSystems/Ohm/Ohm_Pulsse.Ohm_Pulsse" self "/Game/PFX/NiagraSystems/ToBeMade/NS_EchoHit.NS_EchoHit"))

(fn `Damage Effect`
  (params (NewParam :type "Actor Object Reference")))

(fn `Interrupted!!`
  (`parent.Interrupted!!`)
  (set `self.swing can damage` false)
  (set `self.IsRolling` false)
  (set `self.can unroll(check)` false))

(fn `UserConstructionScript`
  (`parent.UserConstructionScript`)
  (set `self.Fann Scale` 1.3))