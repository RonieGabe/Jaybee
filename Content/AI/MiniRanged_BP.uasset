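; Ranged mini enemy AI that turns to face the player, fires orb projectiles and takes damage.
; A looping FacePlayer event smoothly rotates yaw while the player is visible.
; ShootCycle alternates single and double shoot montages with randomized cooldowns, while a separate event spawns the orb and muzzle effect.
; Damage plays a hurt montage and updates health through shared logic; an unreferenced dash macro is also present.
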(event `self.ReceiveBeginPlay`
  (`|ExecutionSequence`
    (:`then_1`
      (`KismetSystemLibrary.Delay` 0.2)
      (`self.Face Player`))))

(event `Face Player`
  (bind (_returnvalue_roll _returnvalue_pitch _returnvalue_yaw) (`KismetMathLibrary.BreakRotator` (`KismetMathLibrary.RInterpTo` (`self.K2_GetActorRotation`) (`KismetMathLibrary.FindLookAtRotation` (`self.K2_GetActorLocation`) (`self.K2_GetActorLocation` (`GameplayStatics.GetPlayerCharacter` 0))) (`GameplayStatics.GetWorldDeltaSeconds`) 10.0)))
  (if (`self.can seeplayer`)
    (`self.K2_SetActorRotation` (`KismetMathLibrary.MakeRotator` 0.0 0.0 _returnvalue_yaw))
    (`KismetSystemLibrary.Delay` 0.01)
    (`self.Face Player`)))

(event `Shoot Cycle`
  (bind _mesh (`self.Mesh`))
  (if (`self.can seeplayer`)
    (`/Engine/EditorBlueprintResources/StandardMacros.DoOnce` false :!label _label
      (:`Completed`
        (`|PlayMontage` _mesh "/Game/AI/Minis/Shoot_Montage.Shoot_Montage" (`KismetMathLibrary.RandomFloatInRange` 0.9 1.1)
          (:`OnCompleted`
            (`/Engine/EditorBlueprintResources/StandardMacros.FlipFlop`
              (:`A`
                _)
              (:`B`
                (`|PlayMontage` _mesh "/Game/AI/Minis/Shoot_Montage.Shoot_Montage" (`KismetMathLibrary.RandomFloatInRange` 0.9 1.1)
                  (:`OnBlendOut`
                    _)
                  (:`OnInterrupted`
                    _)))))
          (:`OnInterrupted`
            _))
        (`KismetSystemLibrary.Delay` (`KismetMathLibrary.RandomFloatInRange` 2.5 3.5))
        (goto _label :!via `Reset`)))))

(event `Shoot Projectile`
  (bind _returnvalue (`SceneComponent.K2_GetComponentLocation` (`self.ShootPoint`)))
  (bind _returnvalue_2 (`|SpawnActorFromClass` "/Game/AI/OrbProjectile.OrbProjectile_C" (`KismetMathLibrary.MakeTransform` _returnvalue (`KismetMathLibrary.Conv_VectorToRotator` (`SceneComponent.GetForwardVector` (`self.CapsuleComponent`)))) "Undefined" "OverrideRootScale" null null))
  (`/Game/AI/OrbProjectile.Set Projectile Values` :`self` _returnvalue_2 :`EnemyOrigin` self)
  (`GameplayStatics.SpawnEmitterAtLocation` "/Game/StarterContent/Particles/P_Explosion.P_Explosion" _returnvalue))

(event `CustomEvent`
  (params (Damage :type "Float (double-precision)") (`Knockback Power` :type "Float (double-precision)") (`Damage Origin` :type "Transform Structure") (`Damage Causer` :type "Actor Object Reference"))
  (`|ExecutionSequence`
    (:`then_0`
      (`|PlayMontage` (`self.Mesh`) "/Game/AI/Minis/HurtMontage.HurtMontage"))
    (:`then_1`
      (`self.Change Health!!` Damage))))

(fn `Change Health!!`
  (params (`(-)Damage  / (+)Healing ` :type "Float (double-precision)"))
  (bind (_new_current_health _healthpercent) (`/Game/GAME_BP/MyLibrary.Change Health(Shared)` (`self.EnemyMax Health`) (`self.Enemy Current Health`) `(-)Damage  / (+)Healing `))
  (set `self.Enemy Current Health` _new_current_health)
  (set `self.Enemy Health Percent` _healthpercent))

(fn `UserConstructionScript`)