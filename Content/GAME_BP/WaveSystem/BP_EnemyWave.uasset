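; BP_EnemyWave is a placeable enemy wave that dispatches its sub-waves to spawn clusters when a manager starts it.
; StartSpawningWave stores the manager, resets the completed count and has each WaveInfo entry's cluster spawn its enemy type, count and delay at a random point.
; A completion check sets the manager's DoneSpawning once CompletedWaves matches the entry count; nothing here increments that count.
; The construction script labels the wave with its display name.
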(event `StartSpawningWave`
  (params (`Manager Parent` :type "/Game/GAME_BP/WaveSystem/BP_WaveManager Object Reference"))
  (set `self.Completed Waves` 0)
  (set `self.Manager Parent` `Manager Parent`)
  (`KismetSystemLibrary.PrintString` (`KismetStringLibrary.Conv_IntToString` (`KismetArrayLibrary.Array_Length` (`self.Wave Info`))))
  (for _array_element (`self.Wave Info`)
    (`self.Spawn Enemies and stuff` _array_element))
  (`KismetSystemLibrary.PrintString` "YESSIR"))

(event `Spawn Enemies and stuff`
  (params (NewParam :type "/Game/GAME_BP/WaveSystem/EnemyWaveInfo Structure") (SpawnerID :type Integer))
  (`/Game/GAME_BP/WaveSystem/SpawnCluster.Spawn at random point` NewParam_PossibleSpawnClusters_18_5EED511948CAA15197C48CB61F7C2ECB NewParam_EnemyType_2_12B5B9164DC3D59C0898509F169FC676 NewParam_NumberofEnemies_9_651BE410476D9B3806BC2B813C93AD20 self NewParam_Delay_12_308807A345DB9E57FF477B9A861DED67))

(event `Check if sub waves are complete`
  (if (== (`KismetArrayLibrary.Array_Length` (`self.Wave Info`)) (`self.Completed Waves`))
    (set `/Game/GAME_BP/WaveSystem/BP_WaveManager.Done Spawning` true (`self.Manager Parent`))
    (`KismetSystemLibrary.PrintString` "WAVE DONE SPAWNING")))

(fn `UserConstructionScript`
  (`TextRenderComponent.K2_SetText` (`self.Wave Label`) (`KismetTextLibrary.Conv_StringToText` (`KismetSystemLibrary.GetDisplayName` self))))