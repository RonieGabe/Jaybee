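; BP_WaveManager runs a sequence of enemy waves once an Avatar_Parent_BP actor first overlaps its spawn trigger.
; It registers with KO_GameMode, then for each wave shows an animated WBP_WaveNumber widget and, after a short delay, tells the EnemyWaves entry to start spawning.
; A completion check advances the wave when spawning is done and no enemies remain alive.
; Running out of waves fires a victory event that only prints a placeholder string.
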(event `self.ReceiveBeginPlay`
  (bind _asko_game_mode (cast `/Game/GAME_BP/KO_GameMode` (`GameplayStatics.GetGameMode`)))
  (set `self.As KO Game Mode` _asko_game_mode))

(event `Display Wave Name`
  (bind _returnvalue (`|CreateWidget` "/Game/UI/CustimWidgets/WBP_WaveNumber.WBP_WaveNumber_C"))
  (`UserWidget.AddToViewport` _returnvalue 2)
  (`/Game/UI/CustimWidgets/WBP_WaveNumber.Set Wave # Text` _returnvalue (`self.current Wave #`))
  (`/Game/UI/CustimWidgets/WBP_WaveNumber.whole Animation` _returnvalue))

(event `self.Spawn Trigger.OnComponentBeginOverlap`
  (params (OverlappedComponent :type "PrimitiveComponent Object Reference") (OtherActor :type "Actor Object Reference") (OtherComp :type "PrimitiveComponent Object Reference") (OtherBodyIndex :type Integer) (bFromSweep :type Boolean) (SweepResult :type "HitResult Structure (by ref)"))
  (cast `/Game/CHARACTER/Avatar_Parent_BP` OtherActor)
  (`/Engine/EditorBlueprintResources/StandardMacros.DoOnce` false
    (:`Completed`
      (set `self.current Wave #` 1)
      (set `/Game/GAME_BP/KO_GameMode.Current Wave Manager` self (`self.As KO Game Mode`))
      (`self.start Current Wave`))))

(event `start Current Wave`
  (bind _output (`|GetArrayItem` (`self.EnemyWaves`) (- (`self.current Wave #`) 1)))
  (set `self.Done Spawning` false)
  (`/Engine/EditorBlueprintResources/StandardMacros.IsValid` _output
    (:`Is Valid`
      (`self.Display Wave Name`)
      (`KismetSystemLibrary.Delay` 3.0)
      (`/Game/GAME_BP/WaveSystem/BP_EnemyWave.StartSpawningWave` _output self))
    (:`Is Not Valid`
      (`self.Waves completed`))))

(event `CheckEnemiesLeft/Wave Complete`
  (if (== (`/Game/GAME_BP/KO_GameMode.Current Enemies Alive` (`self.As KO Game Mode`)) 0)
    (if (`self.Done Spawning`)
      (`/Engine/EditorBlueprintResources/StandardMacros.IncrementInt` (`self.current Wave #`)
        (:`  `
          (`self.start Current Wave`))))))

(event `Waves completed`
  ;[1 1 1] Victory
  (`KismetSystemLibrary.PrintString` "BIG BALLS"))

(fn `UserConstructionScript`)